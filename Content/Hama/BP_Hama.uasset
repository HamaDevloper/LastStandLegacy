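; Hama player character Blueprint that adds third-person camera behavior and debug hotkeys.
; Reversible timelines shorten the spring arm when aiming and mirror its Y socket offset for shoulder swaps, from values cached at BeginPlay.
; Debug keys spawn power-up and perk actors at the scaled forward vector, without adding actor location, or apply self-damage.
; Tick prints stamina from HamaComponent while HealthComponent is valid.
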(event `self.OnAim`
  (params (InAiming :type Boolean))
  (bind _target_arm_length_ref (`self.Target Arm Length Ref`))
  ; Camera
  ;;[0.15 0.08563 0 0.5] Camera Zoom In/Out While in TPP
  (if InAiming
    (bind (_direction _newtrack_0) (`Timeline|CameraZoomTL` :!label _label)
      (:`Update`
        (set `SpringArmComponent.TargetArmLength` (`KismetMathLibrary.Lerp` _target_arm_length_ref (- _target_arm_length_ref (`self.CameraZoom`)) _newtrack_0) (`self.SpringArm`))))
    (else
      (goto _label :!via `Reverse`))))

(event `self.Switchcamera`
  (params (bIsRightShoulderViewChanged :type Boolean))
  (bind (_socket_offset_ref_x _socket_offset_ref_y _socket_offset_ref_z) (`KismetMathLibrary.BreakVector` (`self.Socket Offset Ref`)))
  (bind (_socket_offset_ref_x_2 _socket_offset_ref_y_2) (`KismetMathLibrary.BreakVector` (`self.Socket Offset Ref`)))
  ; Camera
  ;;[0.000151 0.15 0.008675 0.5] SwitchCamera Right/Left
  (if bIsRightShoulderViewChanged
    (bind (_direction _newtrack_0) (`Timeline|SwitchcameraTL` :!label _label_2)
      (:`Update`
        (set `SpringArmComponent.SocketOffset` (`KismetMathLibrary.MakeVector` _socket_offset_ref_x (`KismetMathLibrary.Lerp` _socket_offset_ref_y_2 (* _socket_offset_ref_y_2 -1.0) _newtrack_0) _socket_offset_ref_z) (`self.SpringArm`))))
    (else
      (goto _label_2 :!via `Reverse`))))

(event `self.ReceiveBeginPlay`
  (bind _springarm (`self.SpringArm`))
  (set `self.Socket Offset Ref` (`SpringArmComponent.SocketOffset` _springarm))
  (set `self.Target Arm Length Ref` (`SpringArmComponent.TargetArmLength` _springarm)))

(event `self.ReceiveTick`
  (params (DeltaSeconds :type "Float (single-precision)"))
  ; Comment
  (if (`KismetSystemLibrary.IsValid` (`self.HealthComponent`))
    (`KismetSystemLibrary.PrintString` (`KismetStringLibrary.Conv_DoubleToString` (`HamaComponent.GetStamina` (`self.HamaComponent`))) true true (struct :`G` 0.66 :`B` 1.0 :`A` 1.0) 1.0 "1")))

(event `MaxAmmo`
  (`|SpawnActorFromClass` "/Game/Powers/BP_MaxAmmo.BP_MaxAmmo_C" (`KismetMathLibrary.MakeTransform` (* (`self.GetActorForwardVector`) 500.0) (`self.K2_GetActorRotation`) (1.0 1.0 100.0)) "Undefined" "MultiplyWithRoot" null null)
  (`KismetSystemLibrary.PrintString` "Hello"))

(event `Key|M`
  (params (Key :type "Key Structure"))
  (:`Pressed`
    (`self.MaxAmmo`)))

(event `Nuke`
  (`|SpawnActorFromClass` "/Game/Powers/BP_Nuke.BP_Nuke_C" (`KismetMathLibrary.MakeTransform` (* (`self.GetActorForwardVector`) 500.0) (`self.K2_GetActorRotation`) (1.0 1.0 100.0)) "Undefined" "MultiplyWithRoot" null null))

(event `Key|N`
  (params (Key :type "Key Structure"))
  (:`Pressed`
    (`self.Nuke`)))

(event `Key|P`
  (params (Key :type "Key Structure"))
  (:`Pressed`
    (`self.StartPower`)))

(event `StartPower`
  (`|SpawnActorFromClass` "/Game/Powers/BP_MaxPower.BP_MaxPower_C" (`KismetMathLibrary.MakeTransform` (* (`self.GetActorForwardVector`) 500.0) (`self.K2_GetActorRotation`) (1.0 1.0 100.0)) "Undefined" "MultiplyWithRoot" null null))

(event `Key|B`
  (params (Key :type "Key Structure"))
  (:`Pressed`
    (`self.Bonus`)))

(event `Bonus`
  (`|SpawnActorFromClass` "/Game/Powers/BP_BonusPoints.BP_BonusPoints_C" (`KismetMathLibrary.MakeTransform` (* (`self.GetActorForwardVector`) 500.0) (`self.K2_GetActorRotation`) (1.0 1.0 100.0)) "Undefined" "MultiplyWithRoot" null null))

(event `Key|I`
  (params (Key :type "Key Structure"))
  (:`Pressed`
    (`self.InstaKill`)))

(event `InstaKill`
  (`|SpawnActorFromClass` "/Game/Powers/BP_Instakill.BP_Instakill_C" (`KismetMathLibrary.MakeTransform` (* (`self.GetActorForwardVector`) 500.0) (`self.K2_GetActorRotation`) (1.0 1.0 100.0)) "Undefined" "MultiplyWithRoot" null null))

(event `Key|O`
  (params (Key :type "Key Structure"))
  (:`Pressed`
    (`self.DoublePoint`)))

(event `Key|H`
  (params (Key :type "Key Structure"))
  (:`Pressed`
    (`self.Machine`)))

(event `DoublePoint`
  (`|SpawnActorFromClass` "/Game/Powers/BP_DoublePoint.BP_DoublePoint_C" (`KismetMathLibrary.MakeTransform` (* (`self.GetActorForwardVector`) 500.0) (`self.K2_GetActorRotation`) (1.0 1.0 100.0)) "Undefined" "MultiplyWithRoot" null null))

(event `Key|Backslash`
  (params (Key :type "Key Structure"))
  (:`Pressed`
    (`self.SpawnPerk`)))

(event `Machine`
  (`|SpawnActorFromClass` "/Game/Powers/BP_DeathMachinePower.BP_DeathMachinePower_C" (`KismetMathLibrary.MakeTransform` (* (`self.GetActorForwardVector`) 500.0) (`self.K2_GetActorRotation`) (1.0 1.0 100.0)) "Undefined" "MultiplyWithRoot" null null))

(event `SpawnPerk`
  (`|SpawnActorFromClass` "/Game/Perks/SpawnPoint/BP_PerkSpawnPoint.BP_PerkSpawnPoint_C" (`KismetMathLibrary.MakeTransform` (* (`self.GetActorForwardVector`) 500.0) (`self.K2_GetActorRotation`) (1.0 1.0 100.0)) "Undefined" "MultiplyWithRoot" null null))

(event `Key|Zero`
  (params (Key :type "Key Structure"))
  (:`Pressed`
    (`self.Damge`)))

(event `Damge`
  (`GameplayStatics.ApplyDamage` self 10.0))

(fn `UserConstructionScript`)